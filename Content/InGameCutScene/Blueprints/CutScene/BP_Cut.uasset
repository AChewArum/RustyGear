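; BP_Cut is one shot in an in-game cutscene: a possessable camera rig that travels along an editable spline.
; On first possession it starts fades, shake and a border/text widget, then a timeline drives the spring arm.
; Cinematic options set speed, focus, FOV and rotation: spline-following, look-at or manual.
; At path end, it advances BP_Master's index, possesses the next cut or returns to the character, and optionally self-destroys.
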(event Custom|CurveSpline
  (bind _spline (Variables|Default|GetSpline))
  ;[0 0 0] Spline Settings
  (for _index (range 0 (Spline|GetNumberOfSplinePoints _spline))
    (Spline|SetSplinePointType _spline _index "Curve" true)))

(event Custom|RemoveLastPoint
  (bind _spline (Variables|Default|GetSpline))
  (bind _returnvalue (Spline|GetNumberOfSplinePoints _spline))
  ;[0 0 0] Spline Settings
  (if (> _returnvalue 2)
    (Spline|RemoveSplinePoint (Variables|Default|GetSpline) (- _returnvalue 1) true)))

(event Custom|Req:%20Stop%20Animation
  (bind _mastebpreference (Variables|Default|GetMasteBPReference))
  (bind _spline (Variables|Default|GetSpline))
  (bind _cutactors (Variables|/Game/InGameCutScene/Blueprints/Master/BP_Master.BP_Master_C|GetCutActors _mastebpreference))
  ;[0 0 0] Movement
  (bind _lenght_ (Timeline|Timeline_0 Stop)
    (:Update
      (Variables|Default|SetLenght _lenght_)
      (Variables|Default|SetRotation (Spline|GetRotationatDistanceAlongSpline _spline (Math|Float|Lerp 0.0 (Spline|GetSplineLength _spline) (Variables|Default|GetLenght)) "Local"))
      (Transformation|SetRelativeLocation (Variables|Default|GetSpringArm) (Spline|GetLocationatDistanceAlongSpline _spline (Math|Float|Lerp 0.0 (Spline|GetSplineLength _spline) (Variables|Default|GetLenght)) "Local") false false)
      (Utilities|FlowControl|Sequence
        (:then_0
          (Utilities|UpdateCinematicOption))
        (:then_1
          (if (Variables|Default|GetAnimEnd)
            (Utilities|FlowControl|DoOnce false
              (:Completed
                (Variables|/Game/InGameCutScene/Blueprints/Master/BP_Master.BP_Master_C|SetCutCurrentIndex _mastebpreference (+ (Variables|/Game/InGameCutScene/Blueprints/Master/BP_Master.BP_Master_C|GetCutCurrentIndex _mastebpreference) 1))
                (Default|PlayBorderAnimation (Variables|Default|GetWBPRef) "Reverse" 0.0 1.0)
                (CallFunction|StartCameraFade false)
                (Utilities|FlowControl|Delay (Variables|Default|GetDuration))
                (Pawn|Possess (Game|GetPlayerController 0) (select (== (Utilities|Array|Length _cutactors) (Variables|/Game/InGameCutScene/Blueprints/Master/BP_Master.BP_Master_C|GetCutCurrentIndex _mastebpreference)) (Variables|/Game/InGameCutScene/Blueprints/Master/BP_Master.BP_Master_C|GetCharacter _mastebpreference) (Utilities|Struct|BreakFStruct_Cutscene (Utilities|Array|Get(acopy) _cutactors (Variables|/Game/InGameCutScene/Blueprints/Master/BP_Master.BP_Master_C|GetCutCurrentIndex _mastebpreference)))))
                (Widget|RemovefromParent (Variables|Default|GetWBPRef))
                (CallFunction|StartCameraFade true)
                (if (== (Utilities|Array|Length _cutactors) (Variables|/Game/InGameCutScene/Blueprints/Master/BP_Master.BP_Master_C|GetCutCurrentIndex _mastebpreference))
                  (Default|SimpleMovetoEnd (Variables|Default|GetMasteBPReference)))
                (if (Variables|Default|GetDestroyWhenFinished)
                  (Actor|DestroyActor))))))))))

(event Custom|LinearSpline
  ;[0 0 0] Spline Settings
  (for _index (range 0 (Spline|GetNumberOfSplinePoints (Variables|Default|GetSpline)))
    (Spline|SetSplinePointType (Variables|Default|GetSpline) _index "Linear" true)))

(event Custom|Req:%20Start%20Animation
  (bind _mastebpreference (Variables|Default|GetMasteBPReference))
  (bind _spline (Variables|Default|GetSpline))
  (bind _cutactors (Variables|/Game/InGameCutScene/Blueprints/Master/BP_Master.BP_Master_C|GetCutActors _mastebpreference))
  ;[0 0 0] Movement
  (bind _lenght_ (Timeline|Timeline_0 PlayFromStart)
    (:Update
      (Variables|Default|SetLenght _lenght_)
      (Variables|Default|SetRotation (Spline|GetRotationatDistanceAlongSpline _spline (Math|Float|Lerp 0.0 (Spline|GetSplineLength _spline) (Variables|Default|GetLenght)) "Local"))
      (Transformation|SetRelativeLocation (Variables|Default|GetSpringArm) (Spline|GetLocationatDistanceAlongSpline _spline (Math|Float|Lerp 0.0 (Spline|GetSplineLength _spline) (Variables|Default|GetLenght)) "Local") false false)
      (Utilities|FlowControl|Sequence
        (:then_0
          (Utilities|UpdateCinematicOption))
        (:then_1
          (if (Variables|Default|GetAnimEnd)
            (Utilities|FlowControl|DoOnce false
              (:Completed
                (Variables|/Game/InGameCutScene/Blueprints/Master/BP_Master.BP_Master_C|SetCutCurrentIndex _mastebpreference (+ (Variables|/Game/InGameCutScene/Blueprints/Master/BP_Master.BP_Master_C|GetCutCurrentIndex _mastebpreference) 1))
                (Default|PlayBorderAnimation (Variables|Default|GetWBPRef) "Reverse" 0.0 1.0)
                (CallFunction|StartCameraFade false)
                (Utilities|FlowControl|Delay (Variables|Default|GetDuration))
                (Pawn|Possess (Game|GetPlayerController 0) (select (== (Utilities|Array|Length _cutactors) (Variables|/Game/InGameCutScene/Blueprints/Master/BP_Master.BP_Master_C|GetCutCurrentIndex _mastebpreference)) (Variables|/Game/InGameCutScene/Blueprints/Master/BP_Master.BP_Master_C|GetCharacter _mastebpreference) (Utilities|Struct|BreakFStruct_Cutscene (Utilities|Array|Get(acopy) _cutactors (Variables|/Game/InGameCutScene/Blueprints/Master/BP_Master.BP_Master_C|GetCutCurrentIndex _mastebpreference)))))
                (Widget|RemovefromParent (Variables|Default|GetWBPRef))
                (CallFunction|StartCameraFade true)
                (if (== (Utilities|Array|Length _cutactors) (Variables|/Game/InGameCutScene/Blueprints/Master/BP_Master.BP_Master_C|GetCutCurrentIndex _mastebpreference))
                  (Default|SimpleMovetoEnd (Variables|Default|GetMasteBPReference)))
                (if (Variables|Default|GetDestroyWhenFinished)
                  (Actor|DestroyActor))))))))))

(event Custom|StartCutScene
  ;[0 0 0] Setup Settings
  (Variables|Default|GetMasteBPReference
    (:then
      (CallFunction|StartCameraFade true)
      (bind _returnvalue (UserInterface|CreateWidget "/Game/InGameCutScene/Widgets/WBP_EasyCutScene.WBP_EasyCutScene_C"))
      (Variables|Default|SetWBPRef _returnvalue)
      (UserInterface|Viewport|AddtoViewport (Variables|Default|GetWBPRef) 0)
      (CallFunction|Req:StartAnimation))
    (:else)))

(event Custom|Start%20Camera%20Fade
  (params (Reverse :type Boolean))
  ;[0 0 0] Setup Settings
  (bind _duration (|CameraFadeOptions Reverse)
    (:End
      (Variables|Default|SetDuration _duration))))

(event EventTick
  (params (DeltaSeconds :type Float%20%28single-precision%29))
  (bind _cinematicoption (Variables|CinemaOption|GetCinematicOption))
  (bind _wbpref (Variables|Default|GetWBPRef))
  (bind (_aspectratiospeed _camerashake _camerashakescale) (Utilities|Struct|BreakFStruct_CineOptions _cinematicoption))
  ;[0 0 0] Event Tick
  (if (Class|Pawn|IsControlled)
    (Utilities|FlowControl|DoOnce false
      (:Completed
        (CallFunction|StartCutScene)
        (Utilities|IsValid _wbpref
          (:Is%20Valid
            (Default|PlayBorderAnimation _wbpref "Forward" 0.0 1.0)
            (Utilities|PlayCameraShake _camerashake _camerashakescale "CameraLocal")
            (Variables|/Game/InGameCutScene/Widgets/WBP_EasyCutScene.WBP_EasyCutScene_C|SetAspectRatioSpeed (Variables|Default|GetWBPRef) _aspectratiospeed)))))))

(fn ConstructionScript
  (bind _spline (Variables|Default|GetSpline))
  ;[0 0 0] Spline / Debug
  (Utilities|FlowControl|Sequence
    (:then_0
      (bind _outactors (Actor|GetAllActorsOfClass "/Game/InGameCutScene/Blueprints/Master/BP_Master.BP_Master_C"))
      (if (Utilities|IsValid (Utilities|Array|Get(acopy) _outactors))
        (Variables|Default|SetMasteBPReference (Utilities|Array|Get(acopy) _outactors))
        (else
          (Development|PrintString (Utilities|String|Append "Error In " (Utilities|GetDisplayName self) " Master Blueprint Missing!") true true "(R=1.000000,G=0.730461,B=0.099899,A=1.000000)" 0.2))))
    (:then_1
      (if (Variables|Default|GetDebug)
        (Transformation|SetRelativeLocation (Variables|Default|GetEnd) (+ (Spline|GetLocationatSplinePoint _spline (Spline|GetNumberOfSplinePoints _spline) "Local") (* (Math|Vector|GetUpVector _spline) 5e+01)) false false)))))