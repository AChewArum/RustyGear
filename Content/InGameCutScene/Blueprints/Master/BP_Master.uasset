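; Master actor for in-game cutscenes, started on BeginPlay or when a grounded Player-tagged character enters a trigger box.
; It optionally fades the camera, hands the player controller to a debug pawn or first cut actor, and gives the character a default controller.
; A timeline-driven macro walks the character through waypoint actors, with optional looping and speed override.
; The construction script draws debug lines to flagged cut actors.
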(event Custom|StartAnimation_
  (params (OverlappedActor :type Actor%20Object%20Reference) (OtherActor :type Actor%20Object%20Reference))
  (bind _camerafadeoptions (Variables|Default|GetCameraFadeOptions))
  (bind _camerafadeoptions_2 (Variables|Default|GetCameraFadeOptions))
  (bind (_startanimation _duration _fadeaudio _color) (Utilities|Struct|BreakFStruct_FadeOption _camerafadeoptions))
  (bind (_fadeaudio_2 _color_2) (Utilities|Struct|BreakFStruct_FadeOption _camerafadeoptions_2))
  ;[0 0 0] SetupSettings
  (bind _ascharacter (Utilities|Casting|CastToCharacter OtherActor))
  (if (Actor|ActorHasTag OtherActor "Player")
    (Variables|Default|SetCharacter _ascharacter)
    (if (not (AI|Components|NavMovement|IsFalling (Variables|/Script/Engine.Character|GetCharacterMovement (Variables|Default|GetCharacter))))
      (Utilities|FlowControl|DoOnce false
        (:Completed
          (switch Utilities|FlowControl|Switch|SwitchonEnum_BeginFade _startanimation
            (:NewEnumerator0
              _)
            (:NewEnumerator1
              (CameraFades|StartCameraFade (Game|GetPlayerCameraManager 0) 0.0 1.5 _duration _color _fadeaudio false)
              (Utilities|FlowControl|Delay _duration)))
          (CallFunction|SetCharacterMode)
          (CallFunction|SimpleMovetoStart)
          (Pawn|Possess (Game|GetPlayerController 0) (select (Utilities|IsValid (Variables|Default|GetCutSceneDebugMode)) (Variables|Default|GetCutSceneDebugMode) (Utilities|Struct|BreakFStruct_Cutscene (Utilities|Array|Get(acopy) (Variables|CutScene|GetCutActors)))))
          (Pawn|SpawnDefaultController (Variables|Default|GetCharacter))
          (Class|PlayerCameraManager|SetManualCameraFade (Game|GetPlayerCameraManager 0) (Utilities|Select :Index (Variables|Default|GetStartAnimation%20) :NewEnumerator0 0.0 :NewEnumerator1 1.0) _color_2 _fadeaudio_2))))))

(event Custom|SimpleMoveToEnd
  (bind _character (Variables|Default|GetCharacter))
  (bind _charactermovement (Variables|/Script/Engine.Character|GetCharacterMovement _character))
  ;[0 0 0] SimpleMoveToLogic
  (Variables|/Script/Engine.CharacterMovementComponent|SetMaxWalkSpeed _charactermovement (select (Variables|Default|GetIsEnableSimpleMoveTo) (Variables|Default|GetSavedPlayerSpeed) (Variables|/Script/Engine.CharacterMovementComponent|GetMaxWalkSpeed _charactermovement)))
  (Timeline|SimpleMoveTo Stop
    (:Update
      (Utilities|SimpleMovetoActor) ; enters at execute
    )))

(event Custom|SetCharacterMode
  (bind _returnvalue (Game|GetPlayerCharacter 0))
  (bind _charactermovement (Variables|/Script/Engine.Character|GetCharacterMovement _returnvalue))
  ;[0 0 0] SetCharMode
  (Variables|/Script/Engine.CharacterMovementComponent|SetbRunPhysicsWithNoController _charactermovement true)
  (Pawn|Components|CharacterMovement|SetMovementMode _charactermovement "MOVE_Walking" 0))

(event Custom|SimpleMoveToStart
  ;[0 0 0] SimpleMoveToLogic
  (Utilities|SimpleMovetoActor :!label _label)
  (Timeline|SimpleMoveTo Play
    (:Update
      (goto _label execute))))

(event EventBeginPlay
  (bind _camerafadeoptions (Variables|Default|GetCameraFadeOptions))
  (bind _camerafadeoptions_2 (Variables|Default|GetCameraFadeOptions))
  (bind _triggerbox (Variables|Default|GetTriggerBox))
  (bind (_startanimation _duration _fadeaudio _color) (Utilities|Struct|BreakFStruct_FadeOption _camerafadeoptions))
  (bind (_fadeaudio_2 _color_2) (Utilities|Struct|BreakFStruct_FadeOption _camerafadeoptions_2))
  ;[0 0 0] SetupSettings
  (switch Utilities|FlowControl|Switch|SwitchonEnum_StartAnimation (Variables|Default|GetStartAnimation)
    (:NewEnumerator0
      (switch Utilities|FlowControl|Switch|SwitchonEnum_BeginFade _startanimation
        (:NewEnumerator0
          _)
        (:NewEnumerator1
          (CameraFades|StartCameraFade (Game|GetPlayerCameraManager 0) 0.0 1.5 _duration _color _fadeaudio false)
          (Utilities|FlowControl|Delay _duration)))
      (CallFunction|SetCharacterMode)
      (CallFunction|SimpleMovetoStart)
      (Pawn|Possess (Game|GetPlayerController 0) (select (Utilities|IsValid (Variables|Default|GetCutSceneDebugMode)) (Variables|Default|GetCutSceneDebugMode) (Utilities|Struct|BreakFStruct_Cutscene (Utilities|Array|Get(acopy) (Variables|CutScene|GetCutActors)))))
      (Pawn|SpawnDefaultController (Variables|Default|GetCharacter))
      (Class|PlayerCameraManager|SetManualCameraFade (Game|GetPlayerCameraManager 0) (Utilities|Select :Index (Variables|Default|GetStartAnimation%20) :NewEnumerator0 0.0 :NewEnumerator1 1.0) _color_2 _fadeaudio_2))
    (:NewEnumerator1
      (if (Utilities|IsValid _triggerbox)
        (Collision|BindEventtoOnActorBeginOverlap _triggerbox (delegate Custom|StartAnimation_))))))

(fn ConstructionScript
  ;[0 0 0] Debug
  (for _array_element (Variables|CutScene|GetCutActors)
    (if (.Debug (Utilities|Struct|BreakFStruct_Cutscene _array_element))
      (Rendering|Debug|DrawDebugLine (Transformation|GetActorLocation (.CutActor (Utilities|Struct|BreakFStruct_Cutscene _array_element))) (Transformation|GetActorLocation) (.DebugColor (Utilities|Struct|BreakFStruct_Cutscene _array_element)) 1.0 2.0))))