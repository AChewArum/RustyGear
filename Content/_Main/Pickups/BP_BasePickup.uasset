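; Base pickup actor that notifies players, on the server only, when they enter or leave its range.
; On BeginPlay, StartState either enables mesh physics or calls DisablePhysics, which stops simulation, leaves the mesh query-only and turns off the Sphere's collision.
; Sphere overlaps with Player-tagged actors send SetPickupInfoMessage to that actor.
; Getters expose the pickup type from PickUpInfo and a default orb type and level.
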(event OnComponentBeginOverlap(Sphere)
  (params (OverlappedComponent :type Primitive%20Component%20Object%20Reference) (OtherActor :type Actor%20Object%20Reference) (OtherComp :type Primitive%20Component%20Object%20Reference) (OtherBodyIndex :type Integer) (bFromSweep :type Boolean) (SweepResult :type Hit%20Result%20Structure%20%28by%20ref%29))
  (Networking|SwitchHasAuthority
    (:Authority
      (if (Actor|ActorHasTag OtherActor "Player")
        (Class|INTHeroCharactor|SetPickupInfo(Message) OtherActor self true)))))

(event OnComponentEndOverlap(Sphere)
  (params (OverlappedComponent :type Primitive%20Component%20Object%20Reference) (OtherActor :type Actor%20Object%20Reference) (OtherComp :type Primitive%20Component%20Object%20Reference) (OtherBodyIndex :type Integer))
  (Networking|SwitchHasAuthority
    (:Authority
      (if (Actor|ActorHasTag OtherActor "Player")
        (Class|INTHeroCharactor|SetPickupInfo(Message) OtherActor self false)))))

(event EventBeginPlay
  (if (Variables|Default|GetStartState)
    (Physics|SetSimulatePhysics (Variables|Default|GetStaticMesh) true)
    (else
      (CallFunction|DisablePhysics))))

(event EventDisablePhysics
  (Physics|SetSimulatePhysics (Variables|Default|GetStaticMesh) false)
  (Collision|SetCollisionEnabled (Variables|Default|GetSphere) "QueryOnly")
  (Collision|SetCollisionEnabled (Variables|Default|GetSphere) "NoCollision"))

(fn ConstructionScript)

(fn GetOrbType
  (return "NewEnumerator0" 0))

(fn GetPickupType
  (return (.PickUpType (Utilities|Struct|BreakS_PickupInfo (Variables|Default|GetPickUpInfo)))))