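; Base pickup orb that carries a stat type (attack power, defense, attack speed or max health) and a level, exposed through getters.
; Setup stores this info and picks a matching particle effect, with none assigned for health; BeginPlay defaults to level 1 health.
; Despite its name, SetOrbType toggles an info popup on overlap, creating or destroying a W_ItemInfo widget component with Korean text after a brief delay.
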(event Custom|Setup
  (params (NewParam :type E_OrbTypes%20Enum :default "NewEnumerator0") (Level :type Integer) (OrbName :type Text))
  (Utilities|Struct|SetmembersinS_OrbInfo (Variables|Default|GetOrbInfo) NewParam Level)
  (Effects|Components|ParticleSystem|SetTemplate (Variables|Default|GetParticleSystem) (Utilities|Select :Index NewParam :NewEnumerator0 "/Game/VFX/FXVarietyPack/Particles/P_ky_fireStorm.P_ky_fireStorm" :NewEnumerator1 "/Game/VFX/FXVarietyPack/Particles/P_ky_aquaStorm.P_ky_aquaStorm" :NewEnumerator2 "/Game/VFX/FXVarietyPack/Particles/P_ky_darkStorm.P_ky_darkStorm" :NewEnumerator3 0)))

(event EventBeginPlay
  (CallFunction|Setup "NewEnumerator3" 1))

(event EventSetOrbType
  (params (Overlapped :type Boolean))
  (bind _orbinfo (Variables|Default|GetOrbInfo))
  (bind (_orbtype _level) (Utilities|Struct|BreakS_OrbInfo _orbinfo))
  (Utilities|FlowControl|Delay 0.05)
  (if Overlapped
    (bind _returnvalue (AddComponent|AddWidgetComponent false))
    (Transformation|SetWorldLocation _returnvalue (Transformation|GetWorldLocation (Variables|Default|GetStaticMesh)) false false)
    (bind _asw_item_info (Utilities|Casting|CastToW_ItemInfo (UserInterface|GetUserWidgetObject _returnvalue)))
    (Default|UpdateItemWidget _asw_item_info (Utilities|Select :Index _orbtype :NewEnumerator0 "공격력" :NewEnumerator1 "방어" :NewEnumerator2 "하하" :NewEnumerator3 "최대체력") (Utilities|Text|ToText(Integer) _level) (Utilities|Select :Index _orbtype :NewEnumerator0 "공격력이 증가합니다" :NewEnumerator1 "방어력이 증가합니다" :NewEnumerator2 "몰라" :NewEnumerator3 "최대체력이 증가합니다."))
    (else
      (Components|DestroyComponent _returnvalue))))

(fn ConstructionScript)

(fn GetOrbType
  (params (NewParam :type Boolean))
  (bind _orbinfo (Variables|Default|GetOrbInfo))
  (bind (_orbtype _level) (Utilities|Struct|BreakS_OrbInfo _orbinfo))
  (return _orbtype _level))

(fn GetPickupType
  (return "NewEnumerator0"))