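; Raptor boss enemy Blueprint that announces itself to the player, pursues with AIMoveTo and fights using montage-driven melee, rush, jump and shot attacks.
; FPickAttack sorts player distance into far, middle, close and too-close bands, then range events use percentage rolls to pick pursuit, an attack or a back step.
; Tick smoothly turns it toward the player during combat, and ChargeFinishedAttack spawns BP_Revolver from its head.
; Laser aiming logic is left disconnected.
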(event OnComponentBeginOverlap(Back)
  (params (OverlappedComponent :type Primitive%20Component%20Object%20Reference) (OtherActor :type Actor%20Object%20Reference) (OtherComp :type Primitive%20Component%20Object%20Reference) (OtherBodyIndex :type Integer) (bFromSweep :type Boolean) (SweepResult :type Hit%20Result%20Structure%20%28by%20ref%29))
  ;[1 1 1] PlayerLocation
  (Utilities|IsValid OtherActor
    (:Is%20Valid
      (if (Actor|ActorHasTag OtherActor "Player")
        (Variables|Default|SetWhereBack? true)))))

(event OnComponentEndOverlap(Back)
  (params (OverlappedComponent :type Primitive%20Component%20Object%20Reference) (OtherActor :type Actor%20Object%20Reference) (OtherComp :type Primitive%20Component%20Object%20Reference) (OtherBodyIndex :type Integer))
  ;[1 1 1] PlayerLocation
  (Utilities|IsValid OtherActor
    (:Is%20Valid
      (if (Actor|ActorHasTag OtherActor "Player")
        (Variables|Default|SetWhereBack? false)))))

(event OnComponentBeginOverlap(Side)
  (params (OverlappedComponent :type Primitive%20Component%20Object%20Reference) (OtherActor :type Actor%20Object%20Reference) (OtherComp :type Primitive%20Component%20Object%20Reference) (OtherBodyIndex :type Integer) (bFromSweep :type Boolean) (SweepResult :type Hit%20Result%20Structure%20%28by%20ref%29))
  (Utilities|IsValid OtherActor
    (:Is%20Valid
      (if (Actor|ActorHasTag OtherActor "Player")
        (Variables|Default|SetWhereSide? true)))))

(event OnComponentEndOverlap(Side)
  (params (OverlappedComponent :type Primitive%20Component%20Object%20Reference) (OtherActor :type Actor%20Object%20Reference) (OtherComp :type Primitive%20Component%20Object%20Reference) (OtherBodyIndex :type Integer))
  (Utilities|IsValid OtherActor
    (:Is%20Valid
      (if (Actor|ActorHasTag OtherActor "Player")
        (Variables|Default|SetWhereSide? false)))))

(event Custom|randomevent
  (switch int (Math|Random|RandomIntegerinRange 0 5)
    (:0
      (CallFunction|FrontJump))
    (:1
      (CallFunction|BackStep))
    (:2
      (CallFunction|RushAttack))
    (:3
      (CallFunction|ShotFire))
    (:4
      (CallFunction|SideAttack))
    (:5
      (CallFunction|BackAttack))))

(event Custom|Multi_DefaultAttack
  (params (InSkeletalMeshComponent :type Skeletal%20Mesh%20Component%20Object%20Reference) (MontageToPlay :type Anim%20Montage%20Object%20Reference))
  ;[1 1 1] SetPlayerTarget
  (Animation|Montage|PlayMontage InSkeletalMeshComponent MontageToPlay))

(event Custom|MiddleRange
  ;[1 1 1] RangeSituation
  (if (CallFunction|FPercentage 7e+01)
    (CallFunction|DefaultPursuit)
    (elif (CallFunction|FPercentage 3e+01)
      (CallFunction|BackStep)
      (else
        (CallFunction|RushAttack)))))

(event Custom|FarRange
  ;[1 1 1] RangeSituation
  (if (CallFunction|FPercentage 66.0)
    (CallFunction|DefaultPursuit)
    (else
      (CallFunction|ShotFire))))

(event Custom|BackAttack
  ;[1 1 1] Actions
  (CallFunction|MultiPlayMontage (Variables|Character|GetMesh) "/Game/_Main/AI/Raptor/Anim/Raptor_Attack_Back_Montage.Raptor_Attack_Back_Montage" 1.0 "None"))

(event Custom|NormalAttack
  ;[1 1 1] BaseAttack
  (CallFunction|MultiDefaultAttack (Variables|Character|GetMesh) "/Game/_Main/AI/Raptor/Anim/Raptor_Attack_01_Fix_Montage.Raptor_Attack_01_Fix_Montage"))

(event Custom|FirstMove
  ;[1 1 1] SetPlayerTarget
  (CallFunction|FirstPursuit)
  (Class|INTHeroCharactor|DoBossEntrance(Message) (CallFunction|FGetPlayerTarget) false (Variables|Default|GetBossName)))

(event Custom|SideAttack
  ;[1 1 1] Actions
  (Variables|Default|SetFacingPlayer? false)
  (Transformation|SetActorRotation (Math|Rotator|MakeRotator 0.0 0.0 (.yaw (Math|Rotator|FindLookatRotation (Transformation|GetActorLocation) (Transformation|GetActorLocation (Variables|Default|GetPlayerTarget))))))
  (CallFunction|MultiPlayMontage (Variables|Character|GetMesh) "/Game/_Main/AI/Raptor/Anim/Raptor_Attack_Side_03_Montage.Raptor_Attack_Side_03_Montage" 1.0 "None"))

(event Custom|ShotFire
  ;[1 1 1] Actions
  (CallFunction|MultiPlayMontage (Variables|Character|GetMesh) "/Game/_Main/AI/Raptor/Anim/Raptor_Shot_01_Montage.Raptor_Shot_01_Montage" 1.0 "None"))

(event Custom|FirstPursuit
  ;[1 1 1] SetPlayerTarget
  (AI|AIMoveTo self "0, 0, 0" (Variables|Default|GetPlayerTarget) 1.2e+03 true
    (:OnSuccess
      (CallFunction|FPickAttack 0.0))
    (:OnFail
      (CallFunction|ClearTarget))))

(event Custom|DefaultPursuit
  ;[1 1 1] DefaultPursuit
  (AI|AIMoveTo self "0, 0, 0" (Variables|Default|GetPlayerTarget) 3e+02 true
    (:OnSuccess
      (CallFunction|FPickAttack 0.0))
    (:OnFail
      (Development|PrintString "Hello"))))

(event Custom|laser)

(event Custom|FaceToPlayer
  ;[1 1 1] FacingPlayer
  (Transformation|SetActorRotation (Math|Interpolation|RInterpTo (Transformation|GetActorRotation) (Math|Rotator|FindLookatRotation (Transformation|GetActorLocation) (Transformation|GetActorLocation (Variables|Default|GetPlayerTarget))) (Variables|Default|GetDelta%20Time) 3.0)))

(event Custom|FrontJump
  ;[1 1 1] Actions
  (CallFunction|MultiPlayMontage (Variables|Character|GetMesh) "/Game/_Main/AI/Raptor/Anim/Raptor_Jump_Montage.Raptor_Jump_Montage" 1.0 "None"))

(event Custom|BackStep
  ;[1 1 1] Actions
  (CallFunction|MultiPlayMontage (Variables|Character|GetMesh) "/Game/_Main/AI/Raptor/Anim/Raptor_Jump_Back_Montage.Raptor_Jump_Back_Montage" 1.0 "None"))

(event Custom|CloseRange
  ;[1 1 1] RangeSituation
  (if (CallFunction|FPercentage 3e+01)
    (if (CallFunction|FPercentage 9e+01)
      (CallFunction|SideAttack)
      (else
        (CallFunction|BackStep)))
    (elif (CallFunction|FPercentage 8e+01)
      (CallFunction|NormalAttack)
      (else
        (CallFunction|BackStep)))))

(event Custom|RushAttack
  ;[1 1 1] Actions
  (CallFunction|MultiPlayMontage (Variables|Character|GetMesh) "/Game/_Main/AI/Raptor/Anim/Raptor_Rush_Montage.Raptor_Rush_Montage" 1.0 "None"))

(event EventFlyingSet
  (params (State :type Boolean))
  (bind _charactermovement (Variables|Character|GetCharacterMovement))
  ;[1 1 1] FlyingSEt
  (if State
    (Pawn|Components|CharacterMovement|SetMovementMode _charactermovement "MOVE_Flying" 0)
    (Variables|Default|SetFacingPlayer? false)
    (else
      (Pawn|Components|CharacterMovement|SetMovementMode _charactermovement "MOVE_Falling" 0)
      (Variables|Default|SetFacingPlayer? true))))

(event EventPickAttack
  ;[1 1 1] Pick Attack
  (Variables|Default|SetFacingPlayer? true)
  (Utilities|FlowControl|Delay 1.0)
  (CallFunction|FPickAttack 0.0))

(event EventBossSpecialEffects
  (params (Emmiter :type Particle%20System%20Object%20Reference) (Location :type Vector :default "0, 0, 0") (Rotation :type Rotator :default "0, 0, 0") (Scale :type Vector :default "0, 0, 0") (Sound :type Sound%20Base%20Object%20Reference))
  ;[1 1 1] SpawnEffect
  (Effects|SpawnEmitteratLocation Emmiter Location Rotation Scale)
  (Audio|PlaySoundatLocation Sound Location Rotation 1.0 1.0 0.0 0 0 0))

(event EventChargingAttack
  (params (State :type Boolean))
  ;[1 1 1] ChargeAttack
)

(event EventSetPlayerTarget
  (params (Target :type Actor%20Object%20Reference))
  ;[1 1 1] SetPlayerTarget
  (bind _outactors (Actor|GetAllActorsOfClass "/Game/_Main/Player/BP_PlayerBase.BP_PlayerBase_C"))
  (Variables|Default|SetPlayerTarget (Utilities|Array|Get(acopy) _outactors))
  (Variables|Default|SetIsCombat true)
  (CallFunction|FMovementState "NewEnumerator1")
  (CallFunction|DefaultPursuit)
  (Development|PrintString (Utilities|GetDisplayName (Utilities|Array|Get(acopy) _outactors))))

(event EventTick
  (params (DeltaSeconds :type Float%20%28single-precision%29))
  ;[1 1 1] Tick
  (Variables|Default|SetDelta%20Time DeltaSeconds)
  (Variables|Default|GetPlayerTarget
    (:then
      (if (and (Variables|Default|GetIsCombat) (Variables|Default|GetFacingPlayer?))
        (CallFunction|FacetoPlayer)))
    (:else)))

(event EventGivePlayerDamage
  (params (Object :type Actor%20Object%20Reference) (KnockDown :type Boolean) (Damage :type Float%20%28single-precision%29) (StunTimer :type Float%20%28single-precision%29) (Impulse :type Vector :default "0, 0, 0"))
  ;[1 1 1] Comment
  (Class|INTHeroCharactor|PlayerHit(Message) Object Damage self KnockDown StunTimer Impulse))

(event EventBeginPlay
  ;[1 1 1] BeginPlaySetSpawn
  (Utilities|FlowControl|Sequence
    (:then_0
      (CallFunction|FStartingSpawn (Transformation|GetActorLocation))
      (Variables|Default|SetFacingPlayer? false))
    (:then_1
      (Collision|SetCollisionEnabled (Variables|Default|GetMeleeSphere) "NoCollision"))))

(event EventChargeFinishedAttack
  (params (State :type Boolean))
  ;[1 1 1] ChargeAttack
  (Game|SpawnActorfromClass "/Game/_Main/AI/Raptor/BP_Revolver.BP_Revolver_C" (Math|Transform|MakeTransform (Transformation|GetSocketLocation (Variables|Character|GetMesh) "Raptor_Head") (Math|Rotator|FindLookatRotation (Transformation|GetActorLocation) (Transformation|GetActorLocation (Variables|Default|GetPlayerTarget)))) "Undefined" 0 0))

(fn ConstructionScript
  (|CallParentFunction))

(fn FPlayDeathAnimation
  (Components|Animation|PlayAnimation (Variables|Character|GetMesh) "/Game/_Main/AI/Raptor/Anim/Raptor_Die_Montage.Raptor_Die_Montage" false)
  (Actor|Tick|SetActorTickEnabled false))

(fn FCheckBreak
  (|CallParentFunction)
  (CallFunction|DefaultPursuit))

(fn FPickAttack
  (params (DistanceToPlayer :type Float%20%28single-precision%29))
  (bind _self self)
  (bind _playertarget (Variables|Default|GetPlayerTarget))
  (bind _returnvalue (Transformation|GetDistanceTo _self _playertarget))
  (if (not (Variables|Default|GetIsDead))
    (if (>= _returnvalue (Variables|Default|GetRangeDistance))
      (CallFunction|FarRange)
      (elif (>= _returnvalue (Variables|Default|GetMeleeDistance))
        (CallFunction|MiddleRange)
        (elif (>= _returnvalue (Variables|Default|GetTooCloseDistance))
          (CallFunction|CloseRange)
          (else
            (CallFunction|BackStep)))))))

(fn FOneTest)

(fn FLaserAim)