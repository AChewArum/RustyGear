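; Base enemy character for networked combat, with boss health UI support and empty drop, ranged-attack and death-animation hooks.
; It roams around spawn until given a target, then taunts, chases and picks montage-driven attacks by distance, disengaging when the player is dead or distant.
; Authority-checked sphere overlaps deal damage by attack type.
; Incoming hits apply weak-point bonuses, drain health and a break-stun meter, flash materials and show floating numbers, ending in multicast death.
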(event OnComponentBeginOverlap(MeleeSphere)
  (params (OverlappedComponent :type Primitive%20Component%20Object%20Reference) (OtherActor :type Actor%20Object%20Reference) (OtherComp :type Primitive%20Component%20Object%20Reference) (OtherBodyIndex :type Integer) (bFromSweep :type Boolean) (SweepResult :type Hit%20Result%20Structure%20%28by%20ref%29))
  ;[1 1 1] MeleeAttack
  (Networking|SwitchHasAuthority
    (:Authority
      (if (Actor|ActorHasTag OtherActor "Player")
        (CallFunction|FGetDamage OtherActor)))))

(event Custom|Multi_PlayMontage
  (params (InSkeletalMeshComponent :type Skeletal%20Mesh%20Component%20Object%20Reference) (MontageToPlay :type Anim%20Montage%20Object%20Reference) (PlayRate :type Float%20%28single-precision%29) (StartingSection :type Name))
  (Animation|Montage|PlayMontage InSkeletalMeshComponent MontageToPlay PlayRate 0.0 StartingSection))

(event Custom|multi_death
  ;[1 1 1] EnemyDeath
  (Collision|SetCollisionProfileName (Variables|Default|GetCapsuleComponent) "Ragdoll" true :!class /Script/Engine.PrimitiveComponent)
  (Components|Animation|SetAnimationMode (Variables|Character|GetMesh) "AnimationSingleNode")
  (CallFunction|FPlayDeathAnimation)
  (bind _outactors (Actor|GetAllActorswithTag "enemy"))
  (if (== (Utilities|Array|Length _outactors) 1)
    (Utilities|FlowControl|Delay 2.0)
    (Class|INTSoulController|Victory(Message) (Game|GetPlayerController 0))))

(event Custom|Multi_TargetWidget
  (params (State :type Boolean) (Player :type Actor%20Object%20Reference))
  (bind _targetwidget (Variables|Default|GetTargetWidget))
  ;[1 1 1] TargetingSystem
  (if (Utilities|IsValid (Game|GetInstigatorController Player))
    (if State
      (Development|SetHiddeninGame _targetwidget false false)
      (else
        (Development|SetHiddeninGame _targetwidget true false)))))

(event Custom|Multi_DropItem)

(event Custom|BreakStun
  ;[1 1 1] BreakStun
  (Variables|States|SetCanMove? false)
  (Variables|Default|SetBreaked? true)
  (Variables|Default|SetFacingPlayer? false)
  (Utilities|Time|ClearTimerbyFunctionName 0 "F_CheckBreak")
  (Variables|EnemyInfo|SetBreakMount (Variables|EnemyInfo|GetMaxBreakMount))
  (CallFunction|MultiPlayMontage (Variables|Character|GetMesh) (CallFunction|FGetMontage (Variables|EnemyInfo|GetBreakStunMontage)) 0.0 "None")
  (Utilities|Time|SetTimerbyFunctionName 0 "F_CheckBreak" (Variables|EnemyInfo|GetBreakStunTime)))

(event EventBeginPlay
  ;[1 1 1] Beginplay setup & start roaming
  (Utilities|FlowControl|Sequence
    (:then_0
      (Variables|States|SetSpawnLocation (Transformation|GetActorLocation))
      (Utilities|FlowControl|Delay 0.2)
      (CallFunction|SetRoaming))
    (:then_1
      (Collision|SetCollisionEnabled (Variables|Default|GetMeleeSphere) "NoCollision"))))

(event EventDoSphereOverlap
  (bind _returnvalue (Transformation|GetActorLocation))
  (bind _returnvalue_2 (Transformation|GetActorForwardVector))
  (bind _returnvalue_3 (* _returnvalue_2 2e+02))
  (bind _returnvalue_4 (+ _returnvalue _returnvalue_3))
  ;[1 1 1] HeavyAttack
  (Networking|SwitchHasAuthority
    (:Authority
      (bind _outactors (Collision|SphereOverlapActors _returnvalue_4 1e+02 (Utilities|Array|MakeArray "ObjectTypeQuery3") 0 (Utilities|Array|MakeArray self)))
      (Rendering|Debug|DrawDebugSphere _returnvalue_4 1e+02 12 "(R=0.907196,G=0.469568,B=1.000000,A=1.000000)" 2.0)
      (for _array_element _outactors
        (if (Actor|ActorHasTag _array_element "Player")
          (CallFunction|FGetDamage _array_element))))))

(event EventDoRangeAttack)

(event Game|Damage|EventAnyDamage
  (params (Damage :type Float%20%28single-precision%29) (DamageType :type Damage%20Type%20Object%20Reference) (InstigatedBy :type Controller%20Object%20Reference) (DamageCauser :type Actor%20Object%20Reference))
  ;[1 1 1] Reciving Damage & Death
  (Rendering|Material|SetMaterial (Variables|Character|GetMesh) 0 (Variables|Default|GetHitMaterial))
  (Rendering|Material|SetMaterial (Variables|Character|GetMesh) 1 (Variables|Default|GetHitMaterial))
  (if (Variables|Default|GetBreaked?)
    (Utilities|Time|ClearTimerbyFunctionName 0 "F_CheckBreak")
    (CallFunction|FCheckBreak))
  (Variables|EnemyInfo|SetHealth (- (Variables|EnemyInfo|GetHealth) (select (Variables|Default|GetWeakPoint?) (* Damage 1.5) Damage)))
  (Utilities|FlowControl|Sequence
    (:then_0
      (if (Variables|EnemyInfo|GetIsBoss)
        (Class|INTSoulController|UpdateBossHealthUI(Message) (Game|GetInstigatorController DamageCauser) (/ (Variables|EnemyInfo|GetHealth) (Variables|EnemyInfo|GetMaxHealth))))
      (if (<= (Variables|EnemyInfo|GetHealth) 0.0)
        (CallFunction|Death DamageCauser)))
    (:then_1
      (if (<= (- (Variables|EnemyInfo|GetBreakMount) (select (Variables|Default|GetWeakPoint?) (* Damage 1.5) Damage)) 0.0)
        (CallFunction|BreakStun)
        (else
          (Variables|EnemyInfo|SetBreakMount (- (Variables|EnemyInfo|GetBreakMount) (select (Variables|Default|GetWeakPoint?) (* Damage 1.5) Damage))))))
    (:then_2
      (bind _returnvalue (AddComponent|AddWidgetComponent false))
      (Transformation|SetWorldLocation _returnvalue (Variables|Default|GetHit%20Location) false false)
      (bind _asw_floating_damage (Utilities|Casting|CastToW_FloatingDamage (UserInterface|GetUserWidgetObject _returnvalue)))
      (Rendering|Components|TextRender|SetText (Variables|/Game/_Main/UI/W_FloatingDamage.W_FloatingDamage_C|GetDamageText _asw_floating_damage) (Utilities|Text|ToText(Float) (select (Variables|Default|GetWeakPoint?) (* Damage 1.5) Damage) "HalfToEven"))
      (Appearance|SetColorandOpacity (Variables|/Game/_Main/UI/W_FloatingDamage.W_FloatingDamage_C|GetDamageText _asw_floating_damage) (Utilities|Struct|MakeSlateColor (select false "(R=1.000000,G=0.000000,B=0.000000,A=1.000000)" "(R=1.000000,G=1.000000,B=1.000000,A=1.000000)")) :!class /Script/UMG.TextBlock)
      (UserInterface|Animation|PlayAnimation _asw_floating_damage (Variables|/Game/_Main/UI/W_FloatingDamage.W_FloatingDamage_C|GetFloatAnimation _asw_floating_damage) 0.0 1 "Forward" 1.0 false)
      (Variables|Default|SetWeakPoint? false)
      (Utilities|FlowControl|Delay 0.05)
      (Rendering|Material|SetMaterial (Variables|Character|GetMesh) 0 (Variables|Default|GetNormalMaterial))
      (Rendering|Material|SetMaterial (Variables|Character|GetMesh) 1 (Variables|Default|GetNormalMaterial)))))

(event EventDeath
  (params (Player :type Actor%20Object%20Reference))
  (bind _charactermovement (Variables|Character|GetCharacterMovement))
  ;[1 1 1] EnemyDeath
  (if (not (Variables|States|GetIsDead))
    (Variables|States|SetIsDead true)
    (CallFunction|MultiDeath)
    (Class|Pawn|DetachfromControllerPendingDestroy)
    (Class|CharacterMovementComponent|SetAvoidanceEnabled _charactermovement false)
    (Pawn|Components|CharacterMovement|DisableMovement _charactermovement)
    (Utilities|FlowControl|Delay 5.0)
    (Actor|DestroyActor)))

(event EventToggleTargetWidget
  (params (State :type Boolean) (Player :type Actor%20Object%20Reference))
  ;[1 1 1] TargetingSystem
  (CallFunction|MultiTargetWidget State Player))

(event EventWeakPointHit?
  (params (Causer :type Actor%20Object%20Reference) (HitLocation :type Vector :default "0, 0, 0") (HitName :type Name :default "None"))
  ;[1 1 1] WeakPointCheck
  (Variables|Default|SetHit%20Location HitLocation)
  (for _array_element (Variables|EnemyInfo|GetWeakPointlist)
    (if (Utilities|Name|Equal(Name) HitName _array_element)
      (Variables|Default|SetWeakPoint? true))))

(event EventClearTarget
  ;[1 1 1] Clear the Player Target
  (Variables|States|SetIsCombat false)
  (Actor|Tick|SetActorTickEnabled false)
  (Variables|States|SetPlayerTarget 0)
  (Default|ClearTarget (.AsEnemy%20AIController (Utilities|Casting|CastToEnemyAIController (Pawn|GetController))))
  (AI|AIMoveTo self (Variables|States|GetStartComabtLocation) 0 7e+01 false
    (:OnSuccess
      (CallFunction|SetRoaming))
    (:OnFail
      (Transformation|SetActorLocation (Variables|States|GetSpawnLocation) false false)
      (CallFunction|SetRoaming))))

(event EventSetRoaming
  ;[1 1 1] Roaming
  (if (and (not (Variables|States|GetIsCombat)) (not (Variables|States|GetIsRoaming)))
    (CallFunction|FMovementState "NewEnumerator1")
    (AI|AIMoveTo self (.RandomLocation (AI|Navigation|GetRandomReachablePointinRadius (Variables|States|GetSpawnLocation) 1e+03 0 0)) 0 5.0 false
      (:then
        (Variables|States|SetIsRoaming true))
      (:OnSuccess
        (Variables|States|SetIsRoaming false)
        (Utilities|FlowControl|Delay 3.0)
        (CallFunction|SetRoaming)))))

(event EventSetPlayerTarget
  (params (Target :type Actor%20Object%20Reference))
  ;[1 1 1] Set player Target & Rotation
  (Variables|States|SetPlayerTarget Target)
  (Variables|States|SetIsCombat true)
  (Variables|States|SetIsRoaming false)
  (Actor|Tick|SetActorTickEnabled true)
  (Variables|States|SetStartComabtLocation (Transformation|GetActorLocation))
  (CallFunction|FMovementState "NewEnumerator2")
  (CallFunction|CheckforTaunt)
  (bind _returnvalue (Utilities|Time|SetTimerbyFunctionName 0 "F_DistanceCheck" 2.0 true))
  (Variables|States|SetDistanceHandle _returnvalue))

(event EventTick
  (params (DeltaSeconds :type Float%20%28single-precision%29))
  ;[1 1 1] Set player Target & Rotation
  (if (Variables|States|GetIsCombat)
    (Variables|States|GetPlayerTarget
      (:then
        (Transformation|SetActorRotation (Math|Rotator|MakeRotator 0.0 0.0 (.yaw (Math|Rotator|FindLookatRotation (Transformation|GetActorLocation) (Transformation|GetActorLocation (Variables|States|GetPlayerTarget)))))))
      (:else))))

(event EventChasePlayer
  ;[1 1 1] Chasing Player
  (if (Variables|States|GetIsCombat)
    (AI|AIMoveTo self "0, 0, 0" (Variables|States|GetPlayerTarget) 1.6e+02 true
      (:OnSuccess
        (CallFunction|RunAttackChoices))
      (:OnFail
        (CallFunction|ClearTarget)))))

(event EventRunAttackChoices
  ;[1 1 1] AttackChoices
  (bind _playertarget (Variables|States|GetPlayerTarget)
    (:then
      (bind _dead (Class|INTHeroCharactor|IsDead(Message) _playertarget))
      (if (not _dead)
        (bind _length (CallFunction|FPickAttack (Transformation|GetDistanceTo self (Variables|States|GetPlayerTarget))))
        (Utilities|FlowControl|Delay _length)
        (CallFunction|ChasePlayer)
        (else
          (CallFunction|ClearTarget))))
    (:else
      (CallFunction|ClearTarget))))

(event EventCheckforTaunt
  (bind _tauntmontage (Variables|EnemyInfo|GetTauntMontage))
  (bind _output (CallFunction|FGetMontage _tauntmontage))
  ;[1 1 1] Taunt / Aggro
  (AI|Navigation|StopMovement (Pawn|GetController))
  (if (>= (Transformation|GetDistanceTo self (Variables|States|GetPlayerTarget)) 2e+02)
    (CallFunction|MultiPlayMontage (Variables|Character|GetMesh) _output 0.0 "None")
    (bind _returnvalue (Animation|GetPlayLength _output))
    (Utilities|FlowControl|Delay _returnvalue)
    (CallFunction|ChasePlayer)
    (else
      (CallFunction|ChasePlayer))))

(event EventSetMeleeCollision
  (params (State :type Boolean))
  ;[1 1 1] MeleeAttack
  (if State
    (Collision|SetCollisionEnabled (Variables|Default|GetMeleeSphere) "QueryOnly")
    (else
      (Collision|SetCollisionEnabled (Variables|Default|GetMeleeSphere) "NoCollision"))))

(fn ConstructionScript
  (|CallParentFunction))

(fn FMovementState
  (params (State :type E_AIMovementState%20Enum :default "NewEnumerator0"))
  (bind _walkspeed (Variables|EnemyInfo|GetWalkSpeed))
  (Variables|/Script/Engine.CharacterMovementComponent|SetMaxWalkSpeed (Variables|Character|GetCharacterMovement) (Utilities|Select :Index State :NewEnumerator0 0.0 :NewEnumerator1 _walkspeed :NewEnumerator2 (* _walkspeed (Variables|EnemyInfo|GetSpeedMultiplier)))))

(fn FPickAttack
  (params (DistanceToPlayer :type Float%20%28single-precision%29))
  (bind _specialattackmontage (Variables|EnemyInfo|GetSpecialAttackMontage))
  (bind _rangeattackmontage (Variables|EnemyInfo|GetRangeAttackMontage))
  (bind _lightattackmontage (Variables|EnemyInfo|GetLightAttackMontage))
  (bind _heavyattackmontage (Variables|EnemyInfo|GetHeavyAttackMontage))
  (bind _output (CallFunction|FGetMontage _heavyattackmontage))
  (bind _output_2 (CallFunction|FGetMontage _specialattackmontage))
  (bind _output_3 (CallFunction|FGetMontage _rangeattackmontage))
  (bind _output_4 (CallFunction|FGetMontage _lightattackmontage))
  (if (<= DistanceToPlayer (Variables|EnemyInfo|GetMeleeDistance))
    (if (CallFunction|FPercentage 3e+01)
      (Variables|States|SetAttackTypes "NewEnumerator0")
      (CallFunction|MultiPlayMontage (Variables|Character|GetMesh) _output_4 0.0 "None")
      (bind _returnvalue (Animation|GetPlayLength _output_4))
      (return (+ _returnvalue 0.5))
      (else
        (Variables|States|SetAttackTypes "NewEnumerator1")
        (CallFunction|MultiPlayMontage (Variables|Character|GetMesh) _output 0.0 "None")
        (bind _returnvalue_2 (Animation|GetPlayLength _output))
        (return (+ _returnvalue_2 0.5))))
    (elif (<= DistanceToPlayer (Variables|EnemyInfo|GetRangeDistance))
      (Variables|States|SetAttackTypes "NewEnumerator3")
      (CallFunction|MultiPlayMontage (Variables|Character|GetMesh) _output_2 0.0 "None")
      (bind _returnvalue_3 (Animation|GetPlayLength _output_2))
      (return (+ _returnvalue_3 0.5))
      (else
        (Variables|States|SetAttackTypes "NewEnumerator2")
        (CallFunction|MultiPlayMontage (Variables|Character|GetMesh) _output_3 0.0 "None")
        (bind _returnvalue_4 (Animation|GetPlayLength _output_3))
        (return (+ _returnvalue_4 0.5))))))

(fn FGetMontage
  (params (Montage :type Array%20of%20Anim%20Montage%20Object%20References))
  (return (Utilities|Array|Get(acopy) Montage (Math|Random|RandomIntegerinRange 0 (- (Utilities|Array|Length Montage) 1)))))

(fn FGetDamage
  (params (HitPlayer :type Actor%20Object%20Reference))
  (switch Utilities|FlowControl|Switch|SwitchonE_EnemyAttackTypes (Variables|States|GetAttackTypes)
    (:NewEnumerator0
      (Game|Damage|ApplyDamage HitPlayer (Variables|EnemyInfo|GetLightAttackDamage) 0 self))
    (:NewEnumerator1
      (Game|Damage|ApplyDamage HitPlayer (Variables|EnemyInfo|GetHeavyAttackDamage) 0 self))
    (:NewEnumerator2
      (Game|Damage|ApplyDamage HitPlayer (Variables|EnemyInfo|GetRangeAttackDamage) 0 self))
    (:NewEnumerator3
      (Game|Damage|ApplyDamage HitPlayer (Variables|EnemyInfo|GetSpecialAttackDamage) 0 self))))

(fn FPercentage
  (params (Percent :type Float%20%28single-precision%29))
  (return (select (== Percent 0.0) false (<= (Math|Random|RandomFloatinRange 0.0 1e+02) Percent))))

(fn FGetAttackTypes
  (return (Variables|States|GetAttackTypes)))

(fn FGetCombatState
  (return (Variables|States|GetIsCombat)))

(fn FGetPlayerTarget
  (return (Variables|States|GetPlayerTarget)))

(fn FPlayDeathAnimation)

(fn FDistanceCheck
  (if (>= (Transformation|GetDistanceTo self (Variables|States|GetPlayerTarget)) 1.5e+03)
    (CallFunction|ClearTarget)
    (Utilities|Time|ClearandInvalidateTimerbyHandle (Variables|States|GetDistanceHandle))))

(fn FStartingSpawn
  (params (SpawnLocation :type Vector))
  (Variables|States|SetSpawnLocation SpawnLocation))

(fn FGetImpulse
  (params (Strength :type Float%20%28single-precision%29))
  (bind _returnvalue (Transformation|GetActorLocation))
  (bind _playertarget (Variables|States|GetPlayerTarget))
  (bind _returnvalue_2 (Transformation|GetActorLocation _playertarget))
  (bind _returnvalue_3 (Math|Vector|GetUnitDirection(Vector) _returnvalue _returnvalue_2))
  (return (* (Math|Vector|MakeVector (.x _returnvalue_3) (.y _returnvalue_3) (+ (.z _returnvalue_3) 0.2)) Strength)))

(fn FDestroyParts
  (params (Target :type Primitive%20Component%20Object%20Reference) (Parts :type Primitive%20Component%20Object%20Reference) (Damage :type Float%20%28single-precision%29))
  (for _array_element (Collision|GetOverlappingActors Target "/Game/_Main/Pickups/BP_BasePickup.BP_BasePickup_C" :!class /Script/Engine.PrimitiveComponent)
    _))

(fn FCheckBreak
  (CallFunction|MultiPlayMontage (Variables|Character|GetMesh) (CallFunction|FGetMontage (Variables|EnemyInfo|GetBreakOutMontage)) 0.0 "End")
  (Variables|Default|SetFacingPlayer? true)
  (Variables|States|SetCanMove? true)
  (Variables|Default|SetBreaked? false))

(fn GetSightRadius
  (return (Variables|EnemyInfo|GetSightRadius)))

(fn IsAIDead
  (return (Variables|States|GetIsDead)))