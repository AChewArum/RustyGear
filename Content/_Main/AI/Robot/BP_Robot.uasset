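; Robot boss AI that targets the player, announces itself after its first approach begins, and fights with distance-based attacks.
; FPickAttack sorts distance into bands that randomly choose attack montages or AIMoveTo pursuit, while Tick smoothly turns it toward the player.
; Events deal radial damage, spawn a projectile and send hits through PlayerHitMessage.
; A head-socket laser trace with Niagara beam exists, but its aim timer setup is unconnected.
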(event OnComponentBeginOverlap(Back)
  (params (OverlappedComponent :type Primitive%20Component%20Object%20Reference) (OtherActor :type Actor%20Object%20Reference) (OtherComp :type Primitive%20Component%20Object%20Reference) (OtherBodyIndex :type Integer) (bFromSweep :type Boolean) (SweepResult :type Hit%20Result%20Structure%20%28by%20ref%29))
  ;[1 1 1] PlayerLocation
  (Utilities|IsValid OtherActor
    (:Is%20Valid
      (if (Actor|ActorHasTag OtherActor "Player")
        (Variables|Default|SetWhereBack? true)))))

(event OnComponentEndOverlap(Back)
  (params (OverlappedComponent :type Primitive%20Component%20Object%20Reference) (OtherActor :type Actor%20Object%20Reference) (OtherComp :type Primitive%20Component%20Object%20Reference) (OtherBodyIndex :type Integer))
  ;[1 1 1] PlayerLocation
  (Utilities|IsValid OtherActor
    (:Is%20Valid
      (if (Actor|ActorHasTag OtherActor "Player")
        (Variables|Default|SetWhereBack? false)))))

(event OnComponentEndOverlap(Side)
  (params (OverlappedComponent :type Primitive%20Component%20Object%20Reference) (OtherActor :type Actor%20Object%20Reference) (OtherComp :type Primitive%20Component%20Object%20Reference) (OtherBodyIndex :type Integer))
  (Utilities|IsValid OtherActor
    (:Is%20Valid
      (if (Actor|ActorHasTag OtherActor "Player")
        (Variables|Default|SetWhereSide? false)))))

(event Custom|randomevent
  (switch int (Math|Random|RandomIntegerinRange 1 4)
    (:0
      (CallFunction|Scratch))
    (:1
      (CallFunction|Stomp))
    (:2
      (CallFunction|BackAttack))
    (:3
      (CallFunction|ShotFire))
    (:4
      (CallFunction|Smash))))

(event Custom|Multi_DefaultAttack
  (params (InSkeletalMeshComponent :type Skeletal%20Mesh%20Component%20Object%20Reference) (MontageToPlay :type Anim%20Montage%20Object%20Reference))
  ;[1 1 1] SetPlayerTarget
  (Animation|Montage|PlayMontage InSkeletalMeshComponent MontageToPlay))

(event Custom|MiddleRange
  ;[1 1 1] RangeSituation
  (if (CallFunction|FPercentage 25.0)
    (CallFunction|Scratch)
    (else
      (CallFunction|DefaultPursuit))))

(event Custom|FarRange
  ;[1 1 1] RangeSituation
  (if (CallFunction|FPercentage 25.0)
    (CallFunction|ShotFire)
    (else
      (CallFunction|DefaultPursuit))))

(event Custom|BackAttack
  ;[1 1 1] Actions
  (CallFunction|MultiPlayMontage (Variables|Character|GetMesh) "/Game/_Main/AI/Robot/Anim/Robot_Attack_Back_Montage.Robot_Attack_Back_Montage" 1.0 "None"))

(event Custom|NormalAttack
  ;[1 1 1] BaseAttack
  (CallFunction|MultiDefaultAttack (Variables|Character|GetMesh) (CallFunction|FGetMontage (Utilities|Array|MakeArray 0 0 0))))

(event Custom|FirstMove
  ;[1 1 1] SetPlayerTarget
  (CallFunction|FirstPursuit)
  (Class|INTHeroCharactor|DoBossEntrance(Message) (CallFunction|FGetPlayerTarget) false (Variables|Default|GetBossName)))

(event Custom|ShotFire
  ;[1 1 1] Actions
  (Transformation|SetActorRotation (Math|Rotator|FindLookatRotation (Transformation|GetActorLocation) (Transformation|GetActorLocation (Variables|Default|GetPlayerTarget))))
  (CallFunction|MultiPlayMontage (Variables|Character|GetMesh) "/Game/_Main/AI/Robot/Anim/Robot_Attack_Montage.Robot_Attack_Montage" 1.0 "None")
  (Variables|Default|SetFacingPlayer? true))

(event Custom|FirstPursuit
  ;[1 1 1] SetPlayerTarget
  (AI|AIMoveTo self "0, 0, 0" (Variables|Default|GetPlayerTarget) 1.2e+03 true
    (:OnSuccess
      (CallFunction|FPickAttack 0.0))
    (:OnFail
      (CallFunction|ClearTarget))))

(event Custom|DefaultPursuit
  ;[1 1 1] DefaultPursuit
  (AI|AIMoveTo self "0, 0, 0" (Variables|Default|GetPlayerTarget) 3e+02 true
    (:OnSuccess
      (CallFunction|FPickAttack 0.0))))

(event Custom|laser
  (bind _playertarget (Variables|Default|GetPlayerTarget))
  (bind _mesh (Variables|Character|GetMesh))
  (bind _returnvalue (Transformation|GetActorLocation _playertarget))
  (bind _returnvalue_2 (Transformation|GetSocketLocation _mesh "Head"))
  (bind _returnvalue_3 (Math|Rotator|FindLookatRotation _returnvalue_2 _returnvalue))
  (bind _returnvalue_4 (Math|Transform|MakeTransform _returnvalue_2 _returnvalue_3))
  (bind (_outhit _returnvalue_5) (Collision|LineTraceByChannel _returnvalue_2 (Math|Vector|SelectVector (Variables|Default|GetPlayerLocation) (+ (.location _returnvalue_4) (* (Math|Vector|GetForwardVector (.rotation _returnvalue_4)) 1.01e+07)) (Variables|Default|GetFireLockedOn?)) "TraceTypeQuery2" false 0 "None" true "(R=1.000000,G=0.000000,B=0.000000,A=1.000000)" "(R=0.000000,G=1.000000,B=0.000000,A=1.000000)" 1.0))
  (if _returnvalue_5
    (bind _returnvalue_6 (Niagara|SpawnSystematLocation "/Game/_Main/AI/LaserEmmiter_System.LaserEmmiter_System" (.TraceStart (Collision|BreakHitResult _outhit))))
    (Effects|Components|ParticleSystem|SetVectorParameter _returnvalue_6 "EndPoint" (.Location (Collision|BreakHitResult _outhit)))))

(event Custom|FaceToPlayer
  ;[1 1 1] FacingPlayer
  (Transformation|SetActorRotation (Math|Interpolation|RInterpTo (Transformation|GetActorRotation) (Math|Rotator|FindLookatRotation (Transformation|GetActorLocation) (Transformation|GetActorLocation (Variables|Default|GetPlayerTarget))) (Variables|Default|GetDelta%20Time) 2.0)))

(event Custom|Smash
  ;[1 1 1] Actions
  (CallFunction|MultiPlayMontage (Variables|Character|GetMesh) "/Game/_Main/AI/Robot/Anim/Robot_AttackReverse_Montage.Robot_AttackReverse_Montage" 1.0 "None"))

(event Custom|Scratch
  ;[1 1 1] Actions
  (CallFunction|MultiPlayMontage (Variables|Character|GetMesh) "/Game/_Main/AI/Robot/Anim/Robot_Scratch_Montage.Robot_Scratch_Montage" 1.0 "None"))

(event Custom|CloseRange
  ;[1 1 1] RangeSituation
  (if (CallFunction|FPercentage 26.0)
    (CallFunction|Stomp)
    (elif (CallFunction|FPercentage 5e+01)
      (CallFunction|Scratch)
      (else
        (CallFunction|BackAttack)))))

(event Custom|Stomp
  ;[1 1 1] Actions
  (CallFunction|MultiPlayMontage (Variables|Character|GetMesh) "/Game/_Main/AI/Robot/Anim/Stomp_Montage.Stomp_Montage" 1.0 "None"))

(event EventFlyingSet
  (params (State :type Boolean))
  (bind _charactermovement (Variables|Character|GetCharacterMovement))
  ;[1 1 1] FlyingSEt
  (if State
    (Pawn|Components|CharacterMovement|SetMovementMode _charactermovement "MOVE_Flying" 0)
    (Variables|Default|SetFacingPlayer? false)
    (else
      (Pawn|Components|CharacterMovement|SetMovementMode _charactermovement "MOVE_Falling" 0)
      (Variables|Default|SetFacingPlayer? true))))

(event EventPickAttack
  ;[1 1 1] Pick Attack
  (Variables|Default|SetFacingPlayer? true)
  (Utilities|FlowControl|Delay (Math|Random|RandomFloatinRange 0.5 1.5))
  (CallFunction|FPickAttack 0.0))

(event EventBossSpecialEffects
  (params (Emmiter :type Particle%20System%20Object%20Reference) (Location :type Vector :default "0, 0, 0") (Rotation :type Rotator :default "0, 0, 0") (Scale :type Vector :default "0, 0, 0") (Sound :type Sound%20Base%20Object%20Reference))
  ;[1 1 1] SpawnEffect
  (Effects|SpawnEmitteratLocation Emmiter Location Rotation Scale)
  (Audio|PlaySoundatLocation Sound Location Rotation 1.0 1.0 0.0 0 0 0))

(event EventAreaDamage
  (bind _returnvalue (Transformation|GetActorLocation))
  (bind _outactors (Collision|SphereOverlapActors _returnvalue 3e+02 (Utilities|Array|MakeArray "ObjectTypeQuery3") "/Game/_Main/Player/BP_PlayerBase.BP_PlayerBase_C" (Utilities|Array|MakeArray self)))
  (for _array_element _outactors
    (CallFunction|GivePlayerDamage _array_element false 15.0 0.0 "0, 0, 0"))
  (for _index (range 0 3)
    (Effects|SpawnEmitteratLocation "/Game/VFX/ParticleSystems/Impact_Blank.Impact_Blank" _returnvalue)))

(event EventChargingAttack
  (params (State :type Boolean))
  ;[1 1 1] ChargeAttack
)

(event EventSetPlayerTarget
  (params (Target :type Actor%20Object%20Reference))
  ;[1 1 1] SetPlayerTarget
  (bind _outactors (Actor|GetAllActorsOfClass "/Game/_Main/Player/BP_PlayerBase.BP_PlayerBase_C"))
  (Variables|Default|SetPlayerTarget (Utilities|Array|Get(acopy) _outactors))
  (Variables|Default|SetIsCombat true)
  (Variables|Default|SetStartComabtLocation (Transformation|GetActorLocation))
  (CallFunction|FMovementState "NewEnumerator1")
  (CallFunction|PickAttack))

(event EventTick
  (params (DeltaSeconds :type Float%20%28single-precision%29))
  ;[1 1 1] Tick
  (Variables|Default|SetDelta%20Time DeltaSeconds)
  (Variables|Default|GetPlayerTarget
    (:then
      (if (and (Variables|Default|GetIsCombat) (Variables|Default|GetFacingPlayer?))
        (CallFunction|FacetoPlayer)))
    (:else)))

(event EventGivePlayerDamage
  (params (Object :type Actor%20Object%20Reference) (KnockDown :type Boolean) (Damage :type Float%20%28single-precision%29) (StunTimer :type Float%20%28single-precision%29) (Impulse :type Vector :default "0, 0, 0"))
  ;[1 1 1] Comment
  (Effects|SpawnEmitteratLocation "/Game/AdvancedMagicFX12/Particles/P_ky_hit_dark.P_ky_hit_dark" (Transformation|GetActorLocation (Variables|Default|GetPlayerTarget)))
  (Class|INTHeroCharactor|PlayerHit(Message) Object Damage self KnockDown StunTimer Impulse))

(event EventBeginPlay
  ;[1 1 1] BeginPlaySetSpawn
  (Utilities|FlowControl|Sequence
    (:then_0
      (CallFunction|FStartingSpawn (Transformation|GetActorLocation))
      (Variables|Default|SetFacingPlayer? false))
    (:then_1
      (Collision|SetCollisionEnabled (Variables|Default|GetMeleeSphere) "NoCollision"))))

(event EventChargeFinishedAttack
  (params (State :type Boolean))
  ;[1 1 1] ChargeAttack
  (Variables|Default|SetFacingPlayer? false)
  (Game|SpawnActorfromClass "/Game/_Main/AI/Robot/BP_Rullt.BP_Rullt_C" (Math|Transform|MakeTransform (Transformation|GetSocketLocation (Variables|Character|GetMesh) "Robot_Left_End") (Transformation|GetActorRotation)) "Undefined" self 0))

(fn ConstructionScript
  (|CallParentFunction))

(fn FPlayDeathAnimation
  (Variables|Default|SetFacingPlayer? false)
  (Components|Animation|PlayAnimation (Variables|Character|GetMesh) "/Game/_Main/AI/Robot/Anim/Robot_Death.Robot_Death" false)
  (Actor|Tick|SetActorTickEnabled false))

(fn FCheckBreak
  (|CallParentFunction)
  (CallFunction|DefaultPursuit))

(fn FPickAttack
  (params (DistanceToPlayer :type Float%20%28single-precision%29))
  (bind _self self)
  (bind _playertarget (Variables|Default|GetPlayerTarget))
  (bind _returnvalue (Transformation|GetDistanceTo _self _playertarget))
  (Variables|Default|SetFacingPlayer? false)
  (if (not (Variables|Default|GetIsDead))
    (if (>= _returnvalue (Variables|Default|GetRangeDistance))
      (CallFunction|FarRange)
      (elif (>= _returnvalue (Variables|Default|GetMeleeDistance))
        (CallFunction|MiddleRange)
        (elif (>= _returnvalue (Variables|Default|GetTooCloseDistance))
          (CallFunction|CloseRange)
          (else
            (CallFunction|Scratch)))))))

(fn FOneTest)

(fn FLaserAim
  (bind _playertarget (Variables|Default|GetPlayerTarget))
  (bind _mesh (Variables|Character|GetMesh))
  (bind _returnvalue (Transformation|GetActorLocation _playertarget))
  (bind _returnvalue_2 (Transformation|GetSocketLocation _mesh "Head"))
  (bind _returnvalue_3 (Math|Rotator|FindLookatRotation _returnvalue_2 _returnvalue))
  (bind _returnvalue_4 (Math|Transform|MakeTransform _returnvalue_2 _returnvalue_3))
  (if (Variables|Default|GetFireLockedOn?)
    _
    (else
      (Variables|Default|SetPlayerLocation (+ (.location _returnvalue_4) (* (Math|Vector|GetForwardVector (.rotation _returnvalue_4)) 1.01e+07)))))
  (bind (_outhit _returnvalue_5) (Collision|LineTraceByChannel _returnvalue_2 (Variables|Default|GetPlayerLocation) "TraceTypeQuery2" false 0 "None" true "(R=1.000000,G=0.000000,B=0.000000,A=1.000000)" "(R=0.000000,G=1.000000,B=0.000000,A=1.000000)" 1.0))
  (if _returnvalue_5
    (bind _returnvalue_6 (Niagara|SpawnSystematLocation "/Game/_Main/AI/LaserEmmiter_System.LaserEmmiter_System" (.TraceStart (Collision|BreakHitResult _outhit))))
    (Effects|Components|ParticleSystem|SetVectorParameter _returnvalue_6 "EndPoint" (.Location (Collision|BreakHitResult _outhit)))
    (if (Variables|Default|GetChargeAttackFire)
      (Effects|SpawnEmitteratLocation 0 (.Location (Collision|BreakHitResult _outhit)))
      (Utilities|IsValid (.HitActor (Collision|BreakHitResult _outhit))
        (:Is%20Valid
          (if (Actor|ActorHasTag (.HitActor (Collision|BreakHitResult _outhit)) "Player")
            (Class|INTHeroCharactor|PlayerHit(Message) (.HitActor (Collision|BreakHitResult _outhit)) 3e+01 self true 1.0 (CallFunction|FGetImpulse 2e+02))
            (Variables|Default|SetChargeAttackFire false)))))))