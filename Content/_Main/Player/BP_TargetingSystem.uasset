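; Player lock-on targeting component that toggles camera lock on the nearest living enemy.
; A sphere overlap around the pawn gathers BP_EnemyBase actors, filters out dead ones and picks the closest.
; Message calls lock the pawn's camera and toggle the enemy's target widget, keeping both decoupled from this component.
; A looping timer releases the lock when the target's horizontal distance exceeds the search radius.
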(event Custom|Initialize
  (bind _aspawn (Utilities|Casting|CastToPawn (Components|GetOwner)))
  (bind _output_get (Variables|Default|SetPlayerPawn _aspawn))
  (bind _asplayer_controller (Utilities|Casting|CastToPlayerController (Pawn|GetController _output_get)))
  (Variables|Default|SetPlayerController _asplayer_controller))

(event Custom|LockOnTarget
  (if (not (Variables|Default|GetCurrentlyTargeting))
    (CallFunction|FindTargets)
    (else
      (CallFunction|ToggleCameraLock false))))

(event Custom|FindTargets
  (bind (_outactors _returnvalue) (Collision|SphereOverlapActors (Transformation|GetActorLocation (Variables|Default|GetPlayerPawn)) 1.5e+03 (Utilities|Array|MakeArray "ObjectTypeQuery3") "/Game/_Main/AI/BP_EnemyBase.BP_EnemyBase_C"))
  (if _returnvalue
    (for _array_element _outactors
      (bind _isaidead (Class|INTEnemyAI|IsAIDead(Message) _array_element))
      (if (not _isaidead)
        (Utilities|Array|AddUnique (Variables|Default|GetPotentailTargets) _array_element)))
    (for _array_element_2 (Variables|Default|GetPotentailTargets)
      (if (< (Transformation|GetDistanceTo (Variables|Default|GetPlayerPawn) _array_element_2) (Variables|Default|GetClosestDistance))
        (Variables|Default|SetClosestDistance (Transformation|GetDistanceTo (Variables|Default|GetPlayerPawn) _array_element_2))
        (bind _output_get (Variables|Default|SetLockedTarget _array_element_2))
        (Development|PrintString (Utilities|GetDisplayName _output_get))))
    (Variables|Default|SetClosestDistance 1e+04)
    (Utilities|Array|Clear (Variables|Default|GetPotentailTargets))
    (Variables|Default|GetLockedTarget
      (:then
        (CallFunction|ToggleCameraLock true)
        (bind _returnvalue_2 (Utilities|Time|SetTimerbyEvent (delegate Custom|CheckTargetDistance) 0.25 true))
        (Variables|Default|SetLockHandle _returnvalue_2))
      (:else))))

(event Custom|ToggleCameraLock
  (params (State :type Boolean))
  (bind _returnvalue (Components|GetOwner))
  (bind _playerpawn (Variables|Default|GetPlayerPawn))
  (if State
    (Variables|Default|SetCurrentlyTargeting true)
    (Class|INTHeroCharactor|LockCamera(Message) _playerpawn true (Variables|Default|GetLockedTarget))
    (Class|INTEnemyAI|ToggleTargetWidget(Message) (Variables|Default|GetLockedTarget) true _returnvalue)
    (else
      (Variables|Default|SetCurrentlyTargeting false)
      (Class|INTHeroCharactor|LockCamera(Message) _playerpawn false)
      (Class|INTEnemyAI|ToggleTargetWidget(Message) (Variables|Default|GetLockedTarget) false _returnvalue)
      (Variables|Default|SetLockedTarget 0))))

(event Custom|CheckTargetDistance
  (Variables|Default|GetLockedTarget
    (:then
      (if (> (Transformation|GetHorizontalDistanceTo (Variables|Default|GetPlayerPawn) (Variables|Default|GetLockedTarget)) 1.5e+03)
        (CallFunction|ToggleCameraLock false)
        (Utilities|Time|ClearandInvalidateTimerbyHandle (Variables|Default|GetLockHandle))))
    (:else)))