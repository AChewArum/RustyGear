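; Player controller for a Souls-style game that manages screen flow from main menu through story, pause, death and ending screens.
; On character spawn it possesses a new pawn at the first PlayerStart found, starts looping audio and creates the hidden player HUD.
; Public events forward health, stamina, gauge, potion, pickup and boss-bar updates to Client-prefixed events that drive the HUD.
; Input toggles pause via FlipFlop and advances story or ending scenes.
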(event Custom|Client_ShowPickupName
  (params (State :type Boolean) (Message :type Text))
  (Default|PlayerMessage (Variables|Default|GetPlayer%20UI) State Message))

(event Custom|Client_UpdateHealthUI
  (params (NewHealth :type Float%20%28single-precision%29))
  (Default|UpdateHealthBar (Variables|Default|GetPlayer%20UI) NewHealth))

(event Custom|Client_PotionCount
  (params (Count :type Integer))
  (bind _player_ui (Variables|Default|GetPlayer%20UI))
  (Utilities|IsValid _player_ui
    (:Is%20Valid
      (Default|UpdatePotionBar _player_ui Count))))

(event Custom|Client_TogglePlayerUI
  (params (Condition :type Boolean))
  (bind _player_ui (Variables|Default|GetPlayer%20UI))
  (if Condition
    (Widget|SetVisibility _player_ui "Visible")
    (else
      (Widget|SetVisibility _player_ui "Hidden"))))

(event Custom|CreateStoryUI
  (bind _returnvalue (UserInterface|CreateWidget "/Game/_Main/UI/W_StoryScene.W_StoryScene_C"))
  (bind _output_get (Variables|Default|SetStoryUI _returnvalue))
  (UserInterface|Viewport|AddtoViewport _output_get 0)
  (Default|SetScene _output_get)
  (Variables|Default|SetStoryTime true))

(event Custom|Client_CreateDeathScreenUI
  (Viewport|RemoveAllWidgets)
  (bind _returnvalue (UserInterface|CreateWidget "/Game/_Main/UI/W_DeathScreen.W_DeathScreen_C"))
  (UserInterface|Viewport|AddtoViewport _returnvalue 0))

(event Custom|Client_UpdateStamina
  (params (StaminaPercentage :type Float%20%28single-precision%29))
  (Default|UpdateStaminaBar (Variables|Default|GetPlayer%20UI) StaminaPercentage))

(event Custom|VictoryWidget
  (Viewport|RemoveAllWidgets)
  (bind _returnvalue (UserInterface|CreateWidget "/Game/_Main/UI/W_Ending_Lose.W_Ending_Lose_C"))
  (bind _output_get (Variables|Default|SetEndingUI _returnvalue))
  (Default|SetScene _output_get)
  (Variables|Default|SetEndingTime true))

(event Custom|Client_ToggleBossBar
  (params (InVisibility :type ESlateVisibility%20Enum :default "Visible") (BossName :type Text))
  (bind _player_ui (Variables|Default|GetPlayer%20UI))
  (Utilities|IsValid _player_ui
    (:Is%20Valid
      (Default|ToggleBossBar _player_ui InVisibility BossName))))

(event Custom|Client_UpdateBossHealthUI
  (params (Percent :type Float%20%28single-precision%29))
  (Default|UpdateBossHPBar (Variables|Default|GetPlayer%20UI) Percent))

(event Custom|FirstLoad
  (if (Pawn|IsLocalPlayerController)
    (bind _returnvalue (UserInterface|CreateWidget "/Game/_Main/UI/W_PlayerUI.W_PlayerUI_C"))
    (bind _output_get (Variables|Default|SetPlayer%20UI _returnvalue))
    (UserInterface|Viewport|AddtoViewport _output_get 0)
    (Variables|Default|SetStoryTime false)
    (CallFunction|TogglePlayerUI false)))

(event Custom|Client_UpdateGuageUI
  (params (Guage :type Float%20%28single-precision%29))
  (Default|UpdateGuageBar (Variables|Default|GetPlayer%20UI) Guage))

(event Custom|Charactor%20Spawn
  (params (PlayerController :type Player%20Controller%20Object%20Reference))
  (bind _outactors (Actor|GetAllActorsOfClass "/Script/Engine.PlayerStart"))
  (bind _returnvalue (Game|SpawnActorfromClass (Variables|Default|GetCharactorClass) (Transformation|GetActorTransform (Utilities|Array|Get(acopy) _outactors)) "AlwaysSpawn" 0 0))
  (Utilities|IsValid _returnvalue
    (:Is%20Valid
      (Pawn|Possess PlayerController _returnvalue)
      (Variables|Default|SetbShowMouseCursor false)
      (Audio|PlaySound2D "/Game/Main_Real_Map/loopback_Cue.loopback_Cue" 1.0 1.0 0.0 0 0)
      (CallFunction|FirstLoad))))

(event EventUpdateGuageUI
  (params (Guage :type Float%20%28single-precision%29))
  (CallFunction|ClientUpdateGuageUI Guage))

(event EventUpdatePotionCount
  (params (Count :type Integer))
  (CallFunction|ClientPotionCount Count))

(event EventTogglePlayerUI
  (params (IsVisible :type Boolean))
  (CallFunction|ClientTogglePlayerUI IsVisible))

(event EventShowPickupName
  (params (State :type Boolean) (Name :type Text))
  (CallFunction|ClientShowPickupName State Name))

(event EventUpdateHealthUI
  (params (NewHealth :type Float%20%28single-precision%29))
  (CallFunction|ClientUpdateHealthUI NewHealth))

(event EventUpdateStaminaUI
  (params (Stamina :type Float%20%28single-precision%29))
  (CallFunction|ClientUpdateStamina Stamina))

(event EventFirstLoading
  (CallFunction|FirstLoad))

(event EventDeathScreenUI
  (CallFunction|ClientCreateDeathScreenUI))

(event EventToggleBossBar
  (params (Visibility :type ESlateVisibility%20Enum :default "Visible") (Bossnam :type Text))
  (CallFunction|ClientToggleBossBar Visibility Bossnam))

(event EventUpdateBossHealthUI
  (params (Percent :type Float%20%28single-precision%29))
  (CallFunction|ClientUpdateBossHealthUI Percent))

(event EventBeginPlay
  (if (Pawn|IsLocalPlayerController)
    (Variables|Default|SetbShowMouseCursor false)
    (bind _returnvalue (UserInterface|CreateWidget "/Game/_Main/UI/W_MainMenu.W_MainMenu_C"))
    (bind _output_get (Variables|Default|SetMainMenu _returnvalue))
    (Input|SetInputModeGameandUI (Game|GetPlayerController 0) _output_get "DoNotLock" true)
    (UserInterface|Viewport|AddtoViewport _output_get 0)
    (Utilities|FlowControl|Delay 0.1)
    (Widget|SetKeyboardFocus (Variables|/Game/_Main/UI/W_MainMenu.W_MainMenu_C|GetStartButton _returnvalue))))

(event Input|ActionEvents|InputActionskip
  (params (Key :type Key%20Structure :default "None"))
  (bind _endingui (Variables|Default|GetEndingUI))
  (:Pressed
    (if (Variables|Default|GetStoryTime)
      (Utilities|IsValid (Variables|Default|GetStoryUI)
        (:Is%20Valid
          (Default|SetScene (Variables|Default|GetStoryUI))))
      (elif (Variables|Default|GetEndingTime)
        (Utilities|IsValid _endingui
          (:Is%20Valid
            (Default|SetScene _endingui)))))))

(event Input|ActionEvents|InputActionPause
  (params (Key :type Key%20Structure :default "None"))
  (bind _returnvalue (Game|GetPlayerController 0))
  (:Pressed
    (Utilities|FlowControl|FlipFlop
      (:A
        (bind _returnvalue_2 (UserInterface|CreateWidget "/Game/_Main/UI/W_PauseMenu.W_PauseMenu_C"))
        (Game|SetGamePaused true)
        (Variables|/Script/Engine.PlayerController|SetbShowMouseCursor _returnvalue false)
        (Input|SetInputModeGameandUI (Game|GetPlayerController 0) _returnvalue_2 "DoNotLock" true)
        (UserInterface|Viewport|AddtoViewport _returnvalue_2 0)
        (Utilities|FlowControl|Delay 0.1)
        (Widget|SetKeyboardFocus (Variables|/Game/_Main/UI/W_PauseMenu.W_PauseMenu_C|Getresumebutton _returnvalue_2)))
      (:B
        (Widget|RemovefromParent _returnvalue_2)
        (Game|SetGamePaused false)
        (Variables|/Script/Engine.PlayerController|SetbShowMouseCursor _returnvalue false)))))

(fn ConstructionScript)